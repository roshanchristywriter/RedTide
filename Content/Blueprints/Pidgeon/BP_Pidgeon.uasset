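; BP_Pidgeon is a delivery pigeon that descends from where it spawns, drops off items, then flies away.
; Each Tick moves it vertically by FlightSpeed and tracks the distance in FlightHeight.
; When the height reaches zero it spawns BP_DeliveredItems just below itself and starts climbing.
; At the top of the climb it clears the Pidgeon reference on the first BP_Fisherman found and destroys itself.
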(event EventBeginPlay)

(event Collision|EventActorBeginOverlap
  (params (OtherActor :type Actor%20Object%20Reference)))

(event EventTick
  (params (DeltaSeconds :type Float%20%28single-precision%29))
  (bind _self self)
  (bind _self_2 self)
  (bind _self_3 self)
  ;[1 1 1] Moves the Pidgeon downwards after being spawned
  (if (Variables|Default|GetIsDelivering)
    (Transformation|SetActorLocation _self_3 (- (Transformation|GetActorLocation _self_3) (Math|Vector|MakeVector 0.0 0.0 (* (Utilities|Time|GetWorldDeltaSeconds) (Variables|Default|GetFlightSpeed)))) false false)
    (Variables|Default|SetFlightHeight (- (Variables|Default|GetFlightHeight) (* (Utilities|Time|GetWorldDeltaSeconds) (Variables|Default|GetFlightSpeed))))
    (if (<= (Variables|Default|GetFlightHeight) 0.0)
      (Variables|Default|SetIsDelivering false)
      (Game|SpawnActorfromClass "/Game/Blueprints/Pidgeon/BP_DeliveredItems.BP_DeliveredItems_C" (Math|Transform|MakeTransform (- (Transformation|GetActorLocation _self_2) (Math|Vector|MakeVector 0.0 0.0 15.0)) (Transformation|GetActorRotation _self_2) (Transformation|GetActorScale3D _self_2)) "Undefined" "MultiplyWithRoot" 0 0))
    (else
      (Transformation|SetActorLocation _self (+ (Transformation|GetActorLocation _self) (Math|Vector|MakeVector 0.0 0.0 (* (Utilities|Time|GetWorldDeltaSeconds) (Variables|Default|GetFlightSpeed)))) false false)
      (Variables|Default|SetFlightHeight (+ (* (Utilities|Time|GetWorldDeltaSeconds) (Variables|Default|GetFlightSpeed)) (Variables|Default|GetFlightHeight)))
      (if (>= (Variables|Default|GetFlightHeight) 1e+03)
        (bind _outactors (Actor|GetAllActorsOfClass "/Game/Characters/Fisherman/BP_Fisherman.BP_Fisherman_C"))
        (bind _output_get (Variables|Default|SetPlayer (Utilities|Array|Get(acopy) _outactors)))
        (Variables|/Game/Characters/Fisherman/BP_Fisherman.BP_Fisherman_C|SetPidgeon _output_get 0)
        (Actor|DestroyActor)))))

(fn ConstructionScript)