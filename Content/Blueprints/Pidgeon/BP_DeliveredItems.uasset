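; BP_DeliveredItems is an interactable pickup in the Pidgeon folder that gives BP_Fisherman an item, set to a worm on BeginPlay.
; A sphere overlap shows or hides a hand prompt as the fisherman enters or leaves.
; Interact adds the item's class to the player's ACInventory, refreshes the HUD inventory, flashes the item icon overhead, plays a pickup sound and destroys the actor.
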(event OnComponentBeginOverlap(Sphere)
  (params (OverlappedComponent :type Primitive%20Component%20Object%20Reference) (OtherActor :type Actor%20Object%20Reference) (OtherComp :type Primitive%20Component%20Object%20Reference) (OtherBodyIndex :type Integer) (bFromSweep :type Boolean) (SweepResult :type Hit%20Result%20Structure%20%28by%20ref%29))
  (Utilities|Casting|CastToBP_Fisherman OtherActor)
  (Rendering|SetVisibility (Variables|Default|GetHand) true false))

(event OnComponentEndOverlap(Sphere)
  (params (OverlappedComponent :type Primitive%20Component%20Object%20Reference) (OtherActor :type Actor%20Object%20Reference) (OtherComp :type Primitive%20Component%20Object%20Reference) (OtherBodyIndex :type Integer))
  (Utilities|Casting|CastToBP_Fisherman OtherActor)
  (Rendering|SetVisibility (Variables|Default|GetHand) false false))

(event EventBeginPlay
  (bind _returnvalue (Game|ConstructObjectfromClass "/Game/Blueprints/Items/DA_Item_Worm.DA_Item_Worm_C"))
  (Variables|Default|SetDroppedItem _returnvalue))

(event EventInteract
  (bind _asbp_fisherman (Utilities|Casting|CastToBP_Fisherman (Game|GetPlayerCharacter 0)))
  (Default|AddItem (Variables|/Game/Characters/Fisherman/BP_Fisherman.BP_Fisherman_C|GetAC_Inventory _asbp_fisherman) (Utilities|GetClass (Variables|Default|GetDroppedItem)))
  (bind _asbp_fisherman_2 (Utilities|Casting|CastToBP_Fisherman (Game|GetPlayerCharacter 0)))
  (Default|UpdateInventory (Variables|/Game/UI/W_FishermanHud.W_FishermanHud_C|GetInventory (Variables|/Game/Characters/Fisherman/BP_Fisherman.BP_Fisherman_C|GetHud _asbp_fisherman_2)))
  (Default|ShowOverheadIcon _asbp_fisherman_2 (Variables|/Game/Blueprints/Items/DA_Item.DA_Item_C|GetIcon (Variables|Default|GetDroppedItem)) 1.0)
  (Audio|PlaySound2D "/Engine/VREditor/Sounds/UI/Object_PickUp.Object_PickUp" 1.0 1.0 0.0 0 0)
  (Actor|DestroyActor))

(fn ConstructionScript)