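; BP_DeliveredTasks is an interactable pickup that hands the tasks in its task inventory component to the fisherman player.
; A sphere trigger toggles a Hand prompt while a BP_Fisherman overlaps it.
; On Interact, it copies each task into the player's task inventory, shows an overhead icon, plays a pickup sound and destroys itself.
; BeginPlay also sets DroppedItem to a newly constructed worm item, which this graph never reads.
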(event OnComponentBeginOverlap(Sphere)
  (params (OverlappedComponent :type Primitive%20Component%20Object%20Reference) (OtherActor :type Actor%20Object%20Reference) (OtherComp :type Primitive%20Component%20Object%20Reference) (OtherBodyIndex :type Integer) (bFromSweep :type Boolean) (SweepResult :type Hit%20Result%20Structure%20%28by%20ref%29))
  (Utilities|Casting|CastToBP_Fisherman OtherActor)
  (Rendering|SetVisibility (Variables|Default|GetHand) true false))

(event OnComponentEndOverlap(Sphere)
  (params (OverlappedComponent :type Primitive%20Component%20Object%20Reference) (OtherActor :type Actor%20Object%20Reference) (OtherComp :type Primitive%20Component%20Object%20Reference) (OtherBodyIndex :type Integer))
  (Utilities|Casting|CastToBP_Fisherman OtherActor)
  (Rendering|SetVisibility (Variables|Default|GetHand) false false))

(event EventBeginPlay
  (bind _returnvalue (Game|ConstructObjectfromClass "/Game/Blueprints/Items/DA_Item_Worm.DA_Item_Worm_C"))
  (Variables|Default|SetDroppedItem _returnvalue))

(event EventInteract
  (bind _asbp_fisherman (Utilities|Casting|CastToBP_Fisherman (Game|GetPlayerCharacter 0)))
  (for _array_element (Variables|/Game/Blueprints/Pidgeon/AC_TaskInvetory.AC_TaskInvetory_C|GetContent (Variables|Default|GetAC_TaskInvetory))
    (Default|AddTask (Variables|/Game/Characters/Fisherman/BP_Fisherman.BP_Fisherman_C|GetAC_TaskInvetory _asbp_fisherman) _array_element))
  (Default|ShowOverheadIcon _asbp_fisherman 0 1.0)
  (Audio|PlaySound2D "/Engine/VREditor/Sounds/UI/Object_PickUp.Object_PickUp" 1.0 1.0 0.0 0 0)
  (Actor|DestroyActor))

(fn ConstructionScript)