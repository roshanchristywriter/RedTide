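; Boundary wall actor that keeps the player's BP_Fisherman inside the map area.
; Its Box marks the allowed area: begin overlap clears IsOutMap, while end overlap sets it, and both print a colored status message.
; On exit, the fisherman is teleported to the PlayerLocalion transform, with location converted from the wall's local space and rotation applied unconverted.
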(event OnComponentEndOverlap(Box)
  (params (OverlappedComponent :type Primitive%20Component%20Object%20Reference) (OtherActor :type Actor%20Object%20Reference) (OtherComp :type Primitive%20Component%20Object%20Reference) (OtherBodyIndex :type Integer))
  (bind _player_localion (Variables|Default|GetPlayer_Localion))
  (bind _asbp_fisherman (Utilities|Casting|CastToBP_Fisherman OtherActor))
  (Variables|Default|SetIs_Out_Map%20 true)
  (Development|PrintText "Out of the map area " true true "(R=1.000000,G=0.000000,B=0.000000,A=1.000000)")
  (Transformation|SetActorLocationAndRotation _asbp_fisherman (Math|Transform|TransformLocation (Transformation|GetActorTransform) (.location _player_localion)) (.rotation _player_localion)))

(event OnComponentBeginOverlap(Box)
  (params (OverlappedComponent :type Primitive%20Component%20Object%20Reference) (OtherActor :type Actor%20Object%20Reference) (OtherComp :type Primitive%20Component%20Object%20Reference) (OtherBodyIndex :type Integer) (bFromSweep :type Boolean) (SweepResult :type Hit%20Result%20Structure%20%28by%20ref%29))
  (Utilities|Casting|CastToBP_Fisherman OtherActor)
  (Variables|Default|SetIs_Out_Map%20 false)
  (Development|PrintText "within map limit" true true "(R=0.031250,G=1.000000,B=0.480874,A=1.000000)"))

(fn ConstructionScript)