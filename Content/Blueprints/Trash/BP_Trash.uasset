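; BP_Trash is a collectible trash pickup for the fishing character.
; A sphere overlap shows or hides a hand prompt while a BP_Fisherman is in range.
; Interact adds the trash item to the player's inventory, refreshes the inventory HUD, shows an overhead recycle-bag icon, plays a crumple sound and destroys the actor.
; The construction script gives the cylinder mesh a random shiny color material.
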(event OnComponentBeginOverlap(Sphere)
  (params (OverlappedComponent :type Primitive%20Component%20Object%20Reference) (OtherActor :type Actor%20Object%20Reference) (OtherComp :type Primitive%20Component%20Object%20Reference) (OtherBodyIndex :type Integer) (bFromSweep :type Boolean) (SweepResult :type Hit%20Result%20Structure%20%28by%20ref%29))
  (Utilities|Casting|CastToBP_Fisherman OtherActor)
  (Rendering|SetVisibility (Variables|Default|GetHand) true false))

(event OnComponentEndOverlap(Sphere)
  (params (OverlappedComponent :type Primitive%20Component%20Object%20Reference) (OtherActor :type Actor%20Object%20Reference) (OtherComp :type Primitive%20Component%20Object%20Reference) (OtherBodyIndex :type Integer))
  (Utilities|Casting|CastToBP_Fisherman OtherActor)
  (Rendering|SetVisibility (Variables|Default|GetHand) false false))

(event EventInteract
  (bind _asbp_fisherman (Utilities|Casting|CastToBP_Fisherman (Game|GetPlayerCharacter 0)))
  (Default|AddItem (Variables|/Game/Characters/Fisherman/BP_Fisherman.BP_Fisherman_C|GetAC_Inventory _asbp_fisherman) "/Game/Blueprints/Items/DA_Item_Trash.DA_Item_Trash_C")
  (bind _asbp_fisherman_2 (Utilities|Casting|CastToBP_Fisherman (Game|GetPlayerCharacter 0)))
  (Default|UpdateInventory (Variables|/Game/UI/W_FishermanHud.W_FishermanHud_C|GetInventory (Variables|/Game/Characters/Fisherman/BP_Fisherman.BP_Fisherman_C|GetHud _asbp_fisherman_2)))
  (Default|ShowOverheadIcon _asbp_fisherman_2 "/Game/UI/Img/recycled-bag.recycled-bag" 1.0)
  (Audio|PlaySound2D "/Game/Audio/SoundEffects/MS_Crumple.MS_Crumple" 1.0 1.0 0.0 0 0)
  (Actor|DestroyActor))

(fn ConstructionScript
  (Rendering|Material|SetMaterial (Variables|Default|GetCylinder) 0 (.OutItem (Utilities|Array|Random (Utilities|Array|MakeArray "/Game/Models/UniversalMaterials/MI_Blue_Shiny.MI_Blue_Shiny" "/Game/Models/UniversalMaterials/MI_Green_Shiny.MI_Green_Shiny" "/Game/Models/UniversalMaterials/MI_Red_Shiny.MI_Red_Shiny" "/Game/Models/UniversalMaterials/MI_White_Shiny.MI_White_Shiny")))))