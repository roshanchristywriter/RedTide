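; BP_TrashBin is an interactable trash bin where the player's fisherman throws out trash.
; A sphere overlap shows a billboard while a BP_Fisherman is inside and hides it on exit.
; Interact calls ThrowOutTrash on the player character and feeds the returned number into the Niagara NumberOfParticles variable before activating it, so the burst reflects the result.
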(event OnComponentBeginOverlap(Sphere)
  (params (OverlappedComponent :type Primitive%20Component%20Object%20Reference) (OtherActor :type Actor%20Object%20Reference) (OtherComp :type Primitive%20Component%20Object%20Reference) (OtherBodyIndex :type Integer) (bFromSweep :type Boolean) (SweepResult :type Hit%20Result%20Structure%20%28by%20ref%29))
  (Utilities|Casting|CastToBP_Fisherman OtherActor)
  (Rendering|SetVisibility (Variables|Default|GetBillboard) true false))

(event OnComponentEndOverlap(Sphere)
  (params (OverlappedComponent :type Primitive%20Component%20Object%20Reference) (OtherActor :type Actor%20Object%20Reference) (OtherComp :type Primitive%20Component%20Object%20Reference) (OtherBodyIndex :type Integer))
  (Utilities|Casting|CastToBP_Fisherman OtherActor)
  (Rendering|SetVisibility (Variables|Default|GetBillboard) false false))

(event EventInteract
  (bind _niagara (Variables|Default|GetNiagara))
  (bind _asbp_fisherman (Utilities|Casting|CastToBP_Fisherman (Game|GetPlayerCharacter 0)))
  (bind _numberoftrash (Default|ThrowOutTrash _asbp_fisherman))
  (Class|NiagaraComponent|SetVariableInt _niagara "NumberOfParticles" _numberoftrash)
  (Components|Activation|Activate _niagara false))

(fn ConstructionScript)