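; BP_Casting_Zone marks an area where the player's fishing cast counts as successful.
; Its Sphere overlap events respond only to actors whose class is exactly BP_Bobber_Ghost.
; The ghost entering sets CastSuccess on player 0's BP_Fisherman and prints the ghost's class name for debugging; leaving clears the flag.
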(event OnComponentBeginOverlap(Sphere)
  (params (OverlappedComponent :type Primitive%20Component%20Object%20Reference) (OtherActor :type Actor%20Object%20Reference) (OtherComp :type Primitive%20Component%20Object%20Reference) (OtherBodyIndex :type Integer) (bFromSweep :type Boolean) (SweepResult :type Hit%20Result%20Structure%20%28by%20ref%29))
  (bind _returnvalue (Utilities|GetClass OtherActor))
  (if (== _returnvalue "/Game/Blueprints/Bobber/BP_Bobber_Ghost.BP_Bobber_Ghost_C")
    (bind _asbp_fisherman (Utilities|Casting|CastToBP_Fisherman (Game|GetPlayerCharacter 0)))
    (Variables|/Game/Characters/Fisherman/BP_Fisherman.BP_Fisherman_C|SetCastSuccess _asbp_fisherman true)
    (Development|PrintString (Utilities|GetClassDisplayName _returnvalue))))

(event OnComponentEndOverlap(Sphere)
  (params (OverlappedComponent :type Primitive%20Component%20Object%20Reference) (OtherActor :type Actor%20Object%20Reference) (OtherComp :type Primitive%20Component%20Object%20Reference) (OtherBodyIndex :type Integer))
  (if (== (Utilities|GetClass OtherActor) "/Game/Blueprints/Bobber/BP_Bobber_Ghost.BP_Bobber_Ghost_C")
    (bind _asbp_fisherman (Utilities|Casting|CastToBP_Fisherman (Game|GetPlayerCharacter 0)))
    (Variables|/Game/Characters/Fisherman/BP_Fisherman.BP_Fisherman_C|SetCastSuccess _asbp_fisherman false)))

(event EventBeginPlay)

(event Collision|EventActorBeginOverlap
  (params (OtherActor :type Actor%20Object%20Reference)))

(event EventTick
  (params (DeltaSeconds :type Float%20%28single-precision%29)))

(fn ConstructionScript)