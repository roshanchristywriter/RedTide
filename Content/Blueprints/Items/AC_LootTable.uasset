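; AC_LootTable is a loot table that picks one item class from its Items list, weighted by drop rate.
; DropLoot reads each item's DropRate from class defaults to find the lowest and highest rates, then rolls a random integer between them.
; Items with a rate at or above the roll go into ValidItems, and one random entry is returned, so higher rates qualify more often.
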(fn DropLoot
  (bind _items (Variables|Default|GetItems))
  (bind _validitems (LocalVariables|GetValidItems))
  (bind _output (Utilities|Array|Get(acopy) _items))
  (bind _droprate (Utilities|GetClassDefaults _output))
  (LocalVariables|SetLowestRate _droprate)
  (LocalVariables|SetHighestRate _droprate)
  (for _array_element (Variables|Default|GetItems)
    (if (> (.DropRate (Utilities|GetClassDefaults _array_element)) (LocalVariables|GetHighestRate))
      (LocalVariables|SetHighestRate (.DropRate (Utilities|GetClassDefaults _array_element)))
      (elif (< (.DropRate (Utilities|GetClassDefaults _array_element)) (LocalVariables|GetLowestRate))
        (LocalVariables|SetLowestRate (.DropRate (Utilities|GetClassDefaults _array_element))))))
  (LocalVariables|SetMagicNumber (Math|Random|RandomIntegerinRange (LocalVariables|GetLowestRate) (LocalVariables|GetHighestRate)))
  (for _array_element_2 (Variables|Default|GetItems)
    (if (<= (LocalVariables|GetMagicNumber) (.DropRate (Utilities|GetClassDefaults _array_element_2)))
      (Utilities|Array|Add (LocalVariables|GetValidItems) _array_element_2)))
  (return (Utilities|Array|Get(acopy) _validitems (Math|Random|RandomIntegerinRange 0 (Utilities|Array|LastIndex _validitems)))))