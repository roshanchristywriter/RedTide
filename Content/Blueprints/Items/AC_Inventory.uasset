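; AC_Inventory is an inventory that stores items as slots of item class and quantity.
; AddItem searches Content for a slot whose class-default Name matches the new item's, then increments that stack with no upper limit.
; Unmatched items take a new slot while the count is below Size; otherwise a red "No Empty Inventory Slots" message prints.
; RemoveItem is an empty stub.
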(fn AddItem
  (params (Item :type DA%20Item%20Class%20Reference))
  (bind (_array_element _array_index) (Utilities|Array|ForEachLoopwithBreak (Variables|Default|GetContent) :!label _label)
    (:LoopBody
      (if (Utilities|Enum|Equal(Enum) (.Name (Utilities|GetClassDefaults (.itemclass _array_element))) (.Name (Utilities|GetClassDefaults Item)))
        (LocalVariables|SetFoundSameSlot true)
        (LocalVariables|SetSlotIndex _array_index)
        (goto _label Break)))
    (:Completed
      (if (LocalVariables|GetFoundSameSlot)
        (Utilities|Array|SetArrayElem (Variables|Default|GetContent) (LocalVariables|GetSlotIndex) (Utilities|Struct|MakeFSlotStruct (.itemclass (Utilities|Array|Get(acopy) (Variables|Default|GetContent) (LocalVariables|GetSlotIndex))) (+ (.quantity (Utilities|Array|Get(acopy) (Variables|Default|GetContent) (LocalVariables|GetSlotIndex))) 1)))
        (elif (< (Utilities|Array|Length (Variables|Default|GetContent)) (Variables|Default|GetSize))
          (Utilities|Array|Add (Variables|Default|GetContent) (Utilities|Struct|MakeFSlotStruct Item 1))
          (else
            (Development|PrintString "No Empty Inventory Slots" true true "(R=1.000000,G=0.000000,B=0.019095,A=1.000000)")))))))

(fn RemoveItem
  (params (SlotID :type DA%20Item%20Class%20Reference)))