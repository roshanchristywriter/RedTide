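; BP_Sign is an interactable sign that shows its text in a W_TextBubble widget, filled on BeginPlay.
; A sphere overlap with BP_Fisherman toggles a Hand prompt and an in-range flag, and leaving also hides the bubble.
; Interact reveals the bubble.
; While in range, Tick turns the bubble toward the player's follow camera by matching its yaw plus 180 degrees.
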(event OnComponentBeginOverlap(Sphere)
  (params (OverlappedComponent :type Primitive%20Component%20Object%20Reference) (OtherActor :type Actor%20Object%20Reference) (OtherComp :type Primitive%20Component%20Object%20Reference) (OtherBodyIndex :type Integer) (bFromSweep :type Boolean) (SweepResult :type Hit%20Result%20Structure%20%28by%20ref%29))
  (Utilities|Casting|CastToBP_Fisherman OtherActor)
  (Rendering|SetVisibility (Variables|Default|GetHand) true false)
  (Variables|Default|SetIsInRange true))

(event OnComponentEndOverlap(Sphere)
  (params (OverlappedComponent :type Primitive%20Component%20Object%20Reference) (OtherActor :type Actor%20Object%20Reference) (OtherComp :type Primitive%20Component%20Object%20Reference) (OtherBodyIndex :type Integer))
  (bind _textbubble (Variables|Default|GetTextBubble))
  (Utilities|Casting|CastToBP_Fisherman OtherActor)
  (Rendering|SetVisibility (Variables|Default|GetHand) false false)
  (Variables|Default|SetIsInRange false)
  (if (Variables|/Script/Engine.SceneComponent|GetbVisible _textbubble)
    (Rendering|SetVisibility _textbubble false false)))

(event EventBeginPlay
  (bind _asw_text_bubble (Utilities|Casting|CastToW_TextBubble (UserInterface|GetWidget (Variables|Default|GetTextBubble))))
  (Default|SetText _asw_text_bubble (Variables|Default|GetText)))

(event EventTick
  (params (DeltaSeconds :type Float%20%28single-precision%29))
  (if (Variables|Default|GetIsInRange)
    (bind _asbp_fisherman (Utilities|Casting|CastToBP_Fisherman (Game|GetPlayerCharacter 0)))
    (Transformation|SetWorldRotation (Variables|Default|GetTextBubble) (Math|Rotator|MakeRotator 0.0 0.0 (+ (.yaw (Transformation|GetWorldRotation (Variables|/Game/Characters/Fisherman/BP_Fisherman.BP_Fisherman_C|GetFollowCamera _asbp_fisherman))) 1.8e+02)) false false)))

(event EventInteract
  (Utilities|Casting|CastToBP_Fisherman (Game|GetPlayerCharacter 0))
  (Rendering|SetVisibility (Variables|Default|GetTextBubble) true false))

(fn ConstructionScript)